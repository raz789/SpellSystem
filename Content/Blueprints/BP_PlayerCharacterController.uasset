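; BP_PlayerCharacterController is a player controller that creates the on-screen player UI and hands it the character's modifiers.
; On BeginPlay it casts player pawn 0 to BP_PlayerCharacter and stores that pawn's player modifier array.
; It then creates a BP_PlayerUI widget, adds it to the viewport and initializes it with the stored array.
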(event EventBeginPlay
  (bind _returnvalue (Class|PlayerCharacterController|GetPlayerUIReference))
  (bind _asbp_player_character (Utilities|Casting|CastToBP_PlayerCharacter (Game|Player|GetPlayerPawn 0)))
  (Class|PlayerCharacterController|SetCharacterModifierArray (Class|PlayerCharacter|GetPlayerModifierArray _asbp_player_character))
  (bind _returnvalue_2 (UserInterface|CreateWidget "/Game/Blueprints/UI/BP_PlayerUI.BP_PlayerUI_C" self))
  (Class|PlayerCharacterController|SetPlayerUIReference _returnvalue_2)
  (UserInterface|Viewport|AddtoViewport _returnvalue 0)
  (bind _asbp_player_ui (Utilities|Casting|CastToBP_PlayerUI _returnvalue))
  (Default|Initialize _asbp_player_ui (Class|PlayerCharacterController|GetCharacterModifierArray)))

(event Input|ActionEvents|InputActionUILeftOpen
  (params (Key :type Key%20Structure)))

(fn ConstructionScript)